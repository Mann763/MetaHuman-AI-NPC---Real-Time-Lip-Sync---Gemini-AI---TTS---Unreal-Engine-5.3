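; Base NPC that holds AI-driven, spoken conversations with the player, showing question, state and attitude widgets around a proximity sphere.
; RequestAPI sends the typed question, past dialogue and last attitude tag to Gemini over REST, using a hardcoded API key.
; The reply is split at "^" into dialogue, saved to history and spoken through text-to-speech, and a Friendly/Neutral/Hostile tag for the info widget.
; A polling loop shows Speaking until speech ends.
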(event OnComponentBeginOverlap(Sphere)
  (params (OverlappedComponent :type Primitive%20Component%20Object%20Reference) (OtherActor :type Actor%20Object%20Reference) (OtherComp :type Primitive%20Component%20Object%20Reference) (OtherBodyIndex :type Integer) (bFromSweep :type Boolean) (SweepResult :type Hit%20Result%20Structure%20%28by%20ref%29))
  ;[0 0.1026 1] Hide/Unhide Widget
  (Utilities|Casting|CastToBP_ThirdPersonCharacter OtherActor)
  (CallFunction|ResetWidget)
  (Rendering|SetVisibility (Variables|Default|GetWidget) true false)
  (Rendering|SetVisibility (Variables|Default|GetInfo) true false)
  (CallFunction|ChangeInfo))

(event OnComponentEndOverlap(Sphere)
  (params (OverlappedComponent :type Primitive%20Component%20Object%20Reference) (OtherActor :type Actor%20Object%20Reference) (OtherComp :type Primitive%20Component%20Object%20Reference) (OtherBodyIndex :type Integer))
  ;[0 0.1026 1] Hide/Unhide Widget
  (Utilities|Casting|CastToBP_ThirdPersonCharacter OtherActor)
  (CallFunction|ResetWidget)
  (Rendering|SetVisibility (Variables|Default|GetWidget) false false)
  (Rendering|SetVisibility (Variables|Default|GetState) false false)
  (Rendering|SetVisibility (Variables|Default|GetInfo) false false)
  (CallFunction|ResetInfo))

(event Custom|Request%20API
  (bind _returnvalue (|TexttoSpeechEngineSubsystem))
  (bind _channel_name (Variables|Default|GetChannel%20Name))
  (bind _previousconversations (Variables|Default|GetPreviousConversations))
  ;[0 0.9455 1] Request API Call form Gemini
  (CallFunction|ChangeState true false false true)
  (bind _aswbp_npc (Utilities|Casting|CastToWBP_NPC (UserInterface|GetWidget (Variables|Default|GetWidget))))
  (if (not (Utilities|Text|TextIsEmpty (Variables|/Script/UMG.EditableText|GetText (Variables|/Game/NPC/WBP_NPC.WBP_NPC_C|GetQuestion _aswbp_npc))))
    (if (not (Utilities|Enum|Equal(Enum) (Variables|Default|GetCurrentQuestion) (Utilities|String|ToString(Text) (Variables|/Script/UMG.EditableText|GetText (Variables|/Game/NPC/WBP_NPC.WBP_NPC_C|GetQuestion _aswbp_npc)))))
      (Variables|Default|SetCurrentQuestion (Utilities|String|ToString(Text) (Variables|/Script/UMG.EditableText|GetText (Variables|/Game/NPC/WBP_NPC.WBP_NPC_C|GetQuestion _aswbp_npc))))
      (if (Utilities|Array|IsEmpty (Variables|Default|GetNPC%20Level))
        (Variables|Default|SetNPC%20Level "'This is the first message'"))
      (Variables|Default|SetPreviousChat "")
      (bind _keys (Utilities|Map|Keys _previousconversations))
      (for (_array_element _array_index) _keys
        (Variables|Default|SetTempText (Variables|Default|GetPreviousChat))
        (Variables|Default|SetPreviousChat (Utilities|String|Append (Variables|Default|GetTempText) (Utilities|String|Append (Utilities|String|Append "Player" (Utilities|String|ToString(Integer) _array_index)) ":'" _array_element "'|'NPC: " (.Value (Utilities|Map|Find _previousconversations _array_element)) "' "))))
      (bind (_success _responsecode _data) (Class|RestfulFunctionLibrary|SendRestfulRequest "https://generativelanguage.googleapis.com/v1beta/models/gemini-2.5-flash:generateContent" "POST" (Utilities|String|Append "{ 
    \"contents\": [ 
      { 
        \"parts\": [ 
          {" "\"text\": \"" (Utilities|String|Append "Respond as a game NPC. Keep answers short. No meta-commentary or reactions. Use a status tag at the end: ^[F/N/H][1-5] (Friendly, Neutral, Hostile)Previous " (Variables|Default|GetNPC%20Level) "(Change it based on convo). Evaluate the player's respect level from previous dialogue to determine the tone and respond in the same way. Previous Dialogue:" (Variables|Default|GetPreviousChat) "Current Player Input: '" (Variables|Default|GetCurrentQuestion) ".'") "\"" "          } 
        ] 
      } 
    ] 
  }") (Utilities|Map|MakeMap "x-goog-api-key" "AIzaSyDp4tSb94MjalB4J7vu3qmWYTnjYFOQ5rg" "Content-Type" "application/json") 0.0))
      (if (== _responsecode 200)
        (Utilities|FlowControl|Sequence
          (:then_0
            (bind _outjsonobject (Class|JsonBlueprintFunctionLibrary|FromString _data))
            (bind _outvalue (|GetJsonField _outjsonobject "candidates"))
            (bind _outvalue_2 (|GetJsonField _outvalue "content"))
            (bind _outvalue_3 (|GetJsonField _outvalue_2 "parts"))
            (for _array_element_2 _outvalue_3
              (bind _outvalue_4 (|GetJsonField _array_element_2 "text"))
              (Utilities|Map|Add (Variables|Default|GetPreviousConversations) (Variables|Default|GetCurrentQuestion) (.LeftS (Utilities|String|Split (Utilities|String|Replace _outvalue_4 "\"") "^")))
              (Variables|Default|SetNPC%20Level (.RightS (Utilities|String|Split (Utilities|String|Replace _outvalue_4 "\"") "^")))
              (Class|TexttoSpeechEngineSubsystem|SpeakonChannel _returnvalue _channel_name (.LeftS (Utilities|String|Split (Utilities|String|Replace _outvalue_4 "\"") "^")))
              (if (Class|TexttoSpeechEngineSubsystem|IsSpeakingonChannel _returnvalue _channel_name) :!label _label
                (CallFunction|ChangeState false false true true)
                (Utilities|FlowControl|Delay 0.2)
                (goto _label)
                (else
                  (CallFunction|ChangeState false false false false)))))
          (:then_1
            (bind _aswbp_npc_2 (Utilities|Casting|CastToWBP_NPC (UserInterface|GetWidget (Variables|Default|GetWidget)) :!label _label_2))
            (Variables|/Script/UMG.EditableText|SetText (Variables|/Game/NPC/WBP_NPC.WBP_NPC_C|GetQuestion _aswbp_npc_2) "")
            (Widget|SetVisibility (Variables|/Game/NPC/WBP_NPC.WBP_NPC_C|GetQuestion _aswbp_npc_2) "Collapsed")
            (Widget|SetVisibility (Variables|/Game/NPC/WBP_NPC.WBP_NPC_C|GetAPICall _aswbp_npc_2) "Collapsed")
            (Widget|SetVisibility (Variables|/Game/NPC/WBP_NPC.WBP_NPC_C|GetAsk _aswbp_npc_2) "Visible")))
        (else
          (goto _label_2))))))

(event EventBeginPlay
  (bind _returnvalue (|TexttoSpeechEngineSubsystem))
  (bind _channel_name (Variables|Default|GetChannel%20Name))
  ;[1 0 0] Begin Play
  (Utilities|FlowControl|Sequence
    (:then_0
      (bind _aswbp_npc (Utilities|Casting|CastToWBP_NPC (UserInterface|GetWidget (Variables|Default|GetWidget))))
      (EventDispatchers|AssignOnClicked (Variables|/Game/NPC/WBP_NPC.WBP_NPC_C|GetAPICall _aswbp_npc) (EventDispatchers|CreateEvent :!event Custom|Request%20API)))
    (:then_1
      (Class|TexttoSpeechEngineSubsystem|AddDefaultChannel _returnvalue _channel_name)
      (Class|TexttoSpeechEngineSubsystem|ActivateChannel _returnvalue _channel_name)
      (AI|AIMoveTo (Game|Player|GetPlayerPawn 0) (.RandomLocation (AI|Navigation|GetRandomReachablePointinRadius (Transformation|GetActorLocation) 1e+03 0 0)) self 5.0 false))))

(event Collision|EventActorBeginOverlap
  (params (OtherActor :type Actor%20Object%20Reference)))

(event EventTick
  (params (DeltaSeconds :type Float%20%28single-precision%29)))

(event Input|KeyboardEvents|Enter
  (params (Key :type Key%20Structure :default "None")))

(fn ConstructionScript)

(fn ResetWidget
  (bind _aswbp_npc (Utilities|Casting|CastToWBP_NPC (UserInterface|GetWidget (Variables|Default|GetWidget))))
  (Variables|/Script/UMG.EditableText|SetText (Variables|/Game/NPC/WBP_NPC.WBP_NPC_C|GetQuestion _aswbp_npc) "")
  (Widget|SetVisibility (Variables|/Game/NPC/WBP_NPC.WBP_NPC_C|GetQuestion _aswbp_npc) "Collapsed")
  (Widget|SetVisibility (Variables|/Game/NPC/WBP_NPC.WBP_NPC_C|GetAPICall _aswbp_npc) "Collapsed")
  (Widget|SetVisibility (Variables|/Game/NPC/WBP_NPC.WBP_NPC_C|GetAsk _aswbp_npc) "Visible"))

(fn ChangeState
  (params (Thinking :type Boolean) (Listening :type Boolean) (Speaking :type Boolean) (Activate? :type Boolean))
  (bind _state (Variables|Default|GetState))
  (Utilities|FlowControl|Sequence
    (:then_0
      (if Thinking
        (bind _aswbp_npcstate (Utilities|Casting|CastToWBP_NPCState (UserInterface|GetWidget (Variables|Default|GetState))))
        (Variables|/Script/UMG.EditableTextBox|SetText (Variables|/Game/NPC/WBP_NPCState.WBP_NPCState_C|GetState _aswbp_npcstate) "Thinking…")
        (elif Listening
          (bind _aswbp_npcstate_2 (Utilities|Casting|CastToWBP_NPCState (UserInterface|GetWidget (Variables|Default|GetState))))
          (Variables|/Script/UMG.EditableTextBox|SetText (Variables|/Game/NPC/WBP_NPCState.WBP_NPCState_C|GetState _aswbp_npcstate_2) "Listening…")
          (elif Speaking
            (bind _aswbp_npcstate_3 (Utilities|Casting|CastToWBP_NPCState (UserInterface|GetWidget (Variables|Default|GetState))))
            (Variables|/Script/UMG.EditableTextBox|SetText (Variables|/Game/NPC/WBP_NPCState.WBP_NPCState_C|GetState _aswbp_npcstate_3) "Speaking…")))))
    (:then_1
      (if Activate?
        (Rendering|SetVisibility _state true false)
        (else
          (Rendering|SetVisibility _state false false))))))

(fn ChangeInfo
  (bind _aswbp_npcinfo (Utilities|Casting|CastToWBP_NPCInfo (UserInterface|GetWidget (Variables|Default|GetInfo))))
  (bind _npc_level (CallFunction|GetNPCLevel))
  (Variables|/Script/UMG.EditableTextBox|SetText (Variables|/Game/NPC/WBP_NPCInfo.WBP_NPCInfo_C|GetNHF _aswbp_npcinfo) (Utilities|Text|ToText(String) _npc_level)))

(fn GetNPCLevel
  (bind _npc_level (Variables|Default|GetNPC%20Level))
  (if (or (Utilities|Enum|Equal(Enum) _npc_level "'This is the first message'") (Utilities|Array|IsEmpty _npc_level))
    (return "Neutral")
    (elif (Utilities|String|Contains _npc_level "N")
      (return "Neutral")
      (elif (Utilities|String|Contains _npc_level "H")
        (return "Hostile")
        (elif (Utilities|String|Contains _npc_level "F")
          (return "Friendly"))))))

(fn ResetInfo
  (bind _aswbp_npcinfo (Utilities|Casting|CastToWBP_NPCInfo (UserInterface|GetWidget (Variables|Default|GetInfo))))
  (Widget|SetVisibility (Variables|/Game/NPC/WBP_NPCInfo.WBP_NPCInfo_C|GetIButton _aswbp_npcinfo) "Visible")
  (Widget|SetVisibility (Variables|/Game/NPC/WBP_NPCInfo.WBP_NPCInfo_C|GetInfo _aswbp_npcinfo) "Collapsed"))